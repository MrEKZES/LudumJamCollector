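; BP_MainRocket is a spaceship rocket actor whose parts can be revealed individually.
; The EnableRocketPart event switches on a part type: wings, balon, palkas, engine or front.
; Each case makes the matching component or pair of components visible, without propagating to children.
; It only ever shows parts, with no hiding logic, and its construction script and other events are empty.
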(event Custom|EnableRocketPart
  (params (Parts :type E_PartsOfRocket%20Enum :default "NewEnumerator0"))
  (switch Utilities|FlowControl|Switch|SwitchonE_PartsOfRocket Parts
    (:NewEnumerator0
      (Rendering|SetVisibility (Variables|Default|GetBP_Wing) true false)
      (Rendering|SetVisibility (Variables|Default|GetBP_Wing1) true false))
    (:NewEnumerator1
      (Rendering|SetVisibility (Variables|Default|GetBP_Balon) true false))
    (:NewEnumerator2
      (Rendering|SetVisibility (Variables|Default|GetBP_Palka1) true false)
      (Rendering|SetVisibility (Variables|Default|GetBP_Palka) true false))
    (:NewEnumerator3
      (Rendering|SetVisibility (Variables|Default|GetBP_Engine) true false))
    (:NewEnumerator4
      (Rendering|SetVisibility (Variables|Default|GetBP_Front) true false))))

(event EventBeginPlay)

(event Collision|EventActorBeginOverlap
  (params (OtherActor :type Actor%20Object%20Reference)))

(event EventTick
  (params (DeltaSeconds :type Float%20%28single-precision%29)))

(fn ConstructionScript)