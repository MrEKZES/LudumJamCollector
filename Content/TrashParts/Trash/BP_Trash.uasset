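; BP_Trash is a trash pickup that adds to the player's trash counter when collected.
; On BeginPlay, each instance creates its own WBP_CollectedTrash widget and adds it to the viewport.
; Collect adds a random amount to the passed Player's ITrashCounter, then either clamps it if it exceeds the cap or destroys the actor, so an overflowing pickup remains in the world.
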(event Custom|Collect
  (params (Player :type BP%20Third%20Person%20Character%20Object%20Reference))
  (bind _output_get (Variables|/Game/ThirdPerson/Blueprints/BP_ThirdPersonCharacter.BP_ThirdPersonCharacter_C|SetI_TrashCounter Player (+ (Variables|/Game/ThirdPerson/Blueprints/BP_ThirdPersonCharacter.BP_ThirdPersonCharacter_C|GetI_TrashCounter Player) (Math|Random|RandomIntegerinRange 1 30))))
  (if (> _output_get 100)
    (Variables|/Game/ThirdPerson/Blueprints/BP_ThirdPersonCharacter.BP_ThirdPersonCharacter_C|SetI_TrashCounter Player 100)
    (else
      (Actor|DestroyActor))))

(event EventBeginPlay
  (bind _returnvalue (UserInterface|CreateWidget "/Game/WBP_CollectedTrash.WBP_CollectedTrash_C"))
  (UserInterface|Viewport|AddtoViewport _returnvalue 0))

(fn ConstructionScript)